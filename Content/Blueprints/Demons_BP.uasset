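; Paper2D demon enemy that chases the player until the GameInstance flags game over.
; Tick sweeps it toward the player and picks one of eight directional flipbooks, using look-at pitch in 15-degree buckets and yaw for left or right.
; AnyDamage lowers its health; at zero it fires MonsterDestroyed, shows an explosion, adds score to the GameInstance and destroys itself after a short delay.
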(event Game|Damage|EventAnyDamage
  (params (Damage :type Float%20%28single-precision%29) (DamageType :type Damage%20Type%20Object%20Reference) (InstigatedBy :type Controller%20Object%20Reference) (DamageCauser :type Actor%20Object%20Reference))
  (Variables|Default|SetmonsterHealth (Math|Float|Truncate (- (Math|Conversions|ToFloat(Integer) (Variables|Default|GetmonsterHealth)) Damage))))

(event EventTick
  (params (DeltaSeconds :type Float%20%28single-precision%29))
  (bind _returnvalue (Game|Player|GetPlayerPawn 0))
  (bind _returnvalue_2 (Transformation|GetActorLocation))
  (bind _movementspeed (Variables|Default|GetmovementSpeed))
  (bind _returnvalue_3 (Transformation|GetActorLocation _returnvalue))
  (bind _returnvalue_4 (- _returnvalue_3 _returnvalue_2))
  (bind _returnvalue_5 (Math|Vector|Normalize _returnvalue_4))
  (bind _returnvalue_6 (* _returnvalue_5 DeltaSeconds))
  (bind _returnvalue_7 (* _returnvalue_6 _movementspeed))
  (bind _returnvalue_8 (+ _returnvalue_2 _returnvalue_7))
  (bind (_x _y _z) (Math|Vector|BreakVector _returnvalue_8))
  (bind _returnvalue_9 (Math|Vector|MakeVector _x _y _z))
  ;[1 1 1] Monster Movement
  (if (<= (Variables|Default|GetmonsterHealth) 0)
    ;[1 1 1] Monster destroyed
    (Default|CallMonsterDestroyed)
    (EventDispatchers|UnbindallEventsfromMonsterDestroyed)
    (Sprite|SetFlipbook (Variables|Default|GetPaperFlipbook) "/Game/FlipBooks/Effects/Explosion.Explosion")
    (Utilities|FlowControl|DoOnce false
      (:Completed
        (CallFunction|IncreaseScore)
        (Utilities|FlowControl|Delay 0.1)
        (Actor|DestroyActor)))
    (else
      (bind _asgame_instance_bp (Utilities|Casting|CastToGameInstance_BP (Game|GetGameInstance)))
      (if (not (Variables|/Game/Blueprints/GameInstance_BP.GameInstance_BP_C|GetGameOver _asgame_instance_bp))
        (Transformation|SetActorLocationAndRotation _returnvalue_9 "0, 0, 0" true)
        (bind _viewingdirection (CallFunction|SetViewingDirection (Math|Rotator|FindLookatRotation _returnvalue_9 _returnvalue_3)))
        (Sprite|SetFlipbook (Variables|Default|GetPaperFlipbook) _viewingdirection)))))

(fn ConstructionScript
  ;[1 1 1] Set the flipbook equal to the flipbook of monster we want
  (Sprite|SetFlipbook (Variables|Default|GetPaperFlipbook) (Variables|Default|Getmonster_FB)))

(fn SetViewingDirection
  (params (lookAtRotation :type Rotator))
  (bind (_roll _pitch _yaw) (Math|Rotator|BreakRotator lookAtRotation))
  (bind _returnvalue (/ _pitch 15.0))
  (bind _returnvalue_2 (Math|Float|Floor _returnvalue))
  ;[1 1 1] If Yaw is 180 we are on the left side
  (Math|Float|CompareFloat _yaw 1.8e+02
    (:>
      (Variables|Default|SetfacingLeft true :!label _label))
    (:==
      (goto _label))
    (:<
      (Variables|Default|SetfacingLeft false)))
  ;[1 1 1] Postive values are north, negative south
  (Math|Integer|CompareInt _returnvalue_2 0
    (:>
      (Variables|Default|SetfacingUp true :!label _label_2))
    (:==
      (goto _label_2))
    (:<
      (Variables|Default|SetfacingUp false)))
  (switch int (Math|Integer|Absolute(Integer) _returnvalue_2)
    (:Default
      _)
    (:0
      ;[1 1 1] Facing East/West or Left/Right
      (if (Variables|Default|GetfacingLeft) :!label _label_3
        (return "/Game/FlipBooks/Monsters/Demon_W.Demon_W")
        (else
          (return "/Game/FlipBooks/Monsters/Demon_E.Demon_E"))))
    (:1
      (goto _label_3))
    (:2
      ;[1 1 1] Facing an angle
      (if (Variables|Default|GetfacingUp) :!label _label_4
        ;;[1 1 1] North East or West
        (if (Variables|Default|GetfacingLeft)
          (return "/Game/FlipBooks/Monsters/Demon_NW.Demon_NW")
          (else
            (return "/Game/FlipBooks/Monsters/Demon_NE.Demon_NE")))
        (else
          ;;[1 1 1] South East or West
          (if (Variables|Default|GetfacingLeft)
            (return "/Game/FlipBooks/Monsters/Demon_SW.Demon_SW")
            (else
              (return "/Game/FlipBooks/Monsters/Demon_SE.Demon_SE"))))))
    (:3
      (goto _label_4))
    (:4
      (goto _label_4))
    (:5
      _)
    (:6
      _))
  ;[1 1 1] Facing North/South or Up/Down
  (if (Variables|Default|GetfacingUp)
    (return "/Game/FlipBooks/Monsters/Demon_N.Demon_N")
    (else
      (return "/Game/FlipBooks/Monsters/Demon_S.Demon_S"))))

(fn DestroyMonster)

(fn IncreaseScore
  ;[1 1 1] Increse player score when monster is destroyed
  (bind _asgame_instance_bp (Utilities|Casting|CastToGameInstance_BP (Game|GetGameInstance)))
  (Variables|/Game/Blueprints/GameInstance_BP.GameInstance_BP_C|SetScore _asgame_instance_bp (+ (Variables|/Game/Blueprints/GameInstance_BP.GameInstance_BP_C|GetScore _asgame_instance_bp) 10)))