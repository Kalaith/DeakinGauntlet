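; Paper2D ghost monster that chases the player pawn, loses health from any damage and awards score when killed.
; Tick moves it toward the player with a swept move, and SetViewingDirection maps look-at yaw to one of eight directional ghost flipbooks.
; At zero health, Tick fires and unbinds the MonsterDestroyed dispatcher, shows an explosion, then, behind a DoOnce, adds to the GameInstance_BP score and destroys the actor after a short delay.
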(event Game|Damage|EventAnyDamage
  (params (Damage :type Float%20%28single-precision%29) (DamageType :type Damage%20Type%20Object%20Reference) (InstigatedBy :type Controller%20Object%20Reference) (DamageCauser :type Actor%20Object%20Reference))
  (Variables|Default|SetmonsterHealth (Math|Float|Truncate (- (Math|Conversions|ToFloat(Integer) (Variables|Default|GetmonsterHealth)) Damage))))

(event EventTick
  (params (DeltaSeconds :type Float%20%28single-precision%29))
  (bind _returnvalue (Game|Player|GetPlayerPawn 0))
  (bind _returnvalue_2 (Transformation|GetActorLocation))
  (bind _movementspeed (Variables|Default|GetmovementSpeed))
  (bind _returnvalue_3 (Transformation|GetActorLocation _returnvalue))
  (bind _returnvalue_4 (- _returnvalue_3 _returnvalue_2))
  (bind _returnvalue_5 (Math|Vector|Normalize _returnvalue_4))
  (bind _returnvalue_6 (* _returnvalue_5 DeltaSeconds))
  (bind _returnvalue_7 (* _returnvalue_6 _movementspeed))
  (bind _returnvalue_8 (+ _returnvalue_2 _returnvalue_7))
  (bind (_x _y _z) (Math|Vector|BreakVector _returnvalue_8))
  ;[1 1 1] Monster Movement
  (if (<= (Variables|Default|GetmonsterHealth) 0)
    (Default|CallMonsterDestroyed)
    (EventDispatchers|UnbindallEventsfromMonsterDestroyed)
    (Sprite|SetFlipbook (Variables|Default|GetPaperFlipbook) "/Game/FlipBooks/Effects/Explosion.Explosion")
    (Utilities|FlowControl|DoOnce false
      (:Completed
        (CallFunction|IncreaseScore)
        (Utilities|FlowControl|Delay 0.1)
        (Actor|DestroyActor)))
    (else
      (Transformation|SetActorLocationAndRotation (Math|Vector|MakeVector _x _y _z) "0, 0, 0" true)
      (bind _viewingdirection (CallFunction|SetViewingDirection (Math|Rotator|FindLookatRotation _returnvalue_2 _returnvalue_3)))
      (Sprite|SetFlipbook (Variables|Default|GetPaperFlipbook) _viewingdirection))))

(fn ConstructionScript)

(fn SetViewingDirection
  (params (lookAtRotation :type Rotator))
  (LocalVariables|SetzYaw (.Yaw (Math|Rotator|BreakRotator lookAtRotation)))
  (Math|Float|CompareFloat (LocalVariables|GetzYaw) 0.0
    (:>
      (if (Math|Float|InRange(Float) (LocalVariables|GetzYaw) 0.0 2e+01) :!label _label
        _
        (elif (Math|Float|InRange(Float) (LocalVariables|GetzYaw) 21.0 75.0)
          (bind _output_get (LocalVariables|SetAnimationLocal "/Game/FlipBooks/Monsters/Ghost_SE.Ghost_SE"))
          (return _output_get)
          (elif (Math|Float|InRange(Float) (LocalVariables|GetzYaw) 75.0 115.0)
            (bind _output_get_2 (LocalVariables|SetAnimationLocal "/Game/FlipBooks/Monsters/Ghost_S.Ghost_S"))
            (return _output_get_2)
            (elif (Math|Float|InRange(Float) (LocalVariables|GetzYaw) 116.0 1.6e+02)
              (bind _output_get_3 (LocalVariables|SetAnimationLocal "/Game/FlipBooks/Monsters/Ghost_SW.Ghost_SW"))
              (return _output_get_3)
              (elif (Math|Float|InRange(Float) (LocalVariables|GetzYaw) 161.0 1.8e+02)
                (bind _output_get_4 (LocalVariables|SetAnimationLocal "/Game/FlipBooks/Monsters/Ghost_W.Ghost_W"))
                (return _output_get_4)
                (else
                  (bind _output_get_5 (LocalVariables|SetAnimationLocal "/Game/FlipBooks/Monsters/Ghost_S.Ghost_S" :!label _label_2))
                  (return _output_get_5))))))))
    (:==
      (goto _label))
    (:<
      (LocalVariables|SetzYaw (Math|Float|Absolute(Float) (LocalVariables|GetzYaw)))
      (if (Math|Float|InRange(Float) (LocalVariables|GetzYaw) 0.0 2e+01)
        (bind _output_get_6 (LocalVariables|SetAnimationLocal "/Game/FlipBooks/Monsters/Ghost_E.Ghost_E"))
        (return _output_get_6)
        (elif (Math|Float|InRange(Float) (LocalVariables|GetzYaw) 21.0 75.0)
          (bind _output_get_7 (LocalVariables|SetAnimationLocal "/Game/FlipBooks/Monsters/Ghost_NE.Ghost_NE"))
          (return _output_get_7)
          (elif (Math|Float|InRange(Float) (LocalVariables|GetzYaw) 76.0 115.0)
            (bind _output_get_8 (LocalVariables|SetAnimationLocal "/Game/FlipBooks/Monsters/Ghost_N.Ghost_N"))
            (return _output_get_8)
            (elif (Math|Float|InRange(Float) (LocalVariables|GetzYaw) 116.0 1.6e+02)
              (bind _output_get_9 (LocalVariables|SetAnimationLocal "/Game/FlipBooks/Monsters/Ghost_NW.Ghost_NW"))
              (return _output_get_9)
              (elif (Math|Float|InRange(Float) (LocalVariables|GetzYaw) 161.0 1.8e+02)
                (bind _output_get_10 (LocalVariables|SetAnimationLocal "/Game/FlipBooks/Monsters/Ghost_W.Ghost_W"))
                (return _output_get_10)
                (else
                  (goto _label_2)))))))))
  (bind _output_get_11 (LocalVariables|SetAnimationLocal "/Game/FlipBooks/Monsters/Ghost_E.Ghost_E"))
  (return _output_get_11))

(fn DestroyMonster)

(fn IncreaseScore
  (bind _asgame_instance_bp (Utilities|Casting|CastToGameInstance_BP (Game|GetGameInstance)))
  (Variables|/Game/Blueprints/GameInstance_BP.GameInstance_BP_C|SetScore _asgame_instance_bp (+ (Variables|/Game/Blueprints/GameInstance_BP.GameInstance_BP_C|GetScore _asgame_instance_bp) 10)))