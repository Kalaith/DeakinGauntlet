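; Player Blueprint for a Paper2D elf that moves in eight directions on the X/Z plane and fires projectiles.
; Tick stores the last non-zero input, offsets the actor with sweep unless shooting, and sets a walk or idle flipbook through UpdateAnimation.
; Holding Shoot stops movement while input still steers aim, spawning projectiles with sound along the last direction.
; A CanFire flag reset by a timer limits the fire rate.
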(event EventTick
  (params (DeltaSeconds :type Float%20%28single-precision%29))
  (bind _returnvalue (Input|AxisValues|GetMoveForward))
  (bind _returnvalue_2 (Input|AxisValues|GetMoveRight))
  (bind _movementspeed (Variables|Default|GetMovementSpeed))
  (bind _returnvalue_3 (Math|Vector|MakeVector _returnvalue_2 0.0 _returnvalue))
  (bind _returnvalue_4 (* DeltaSeconds _movementspeed))
  (bind _returnvalue_5 (Math|Vector|ClampVectorSize _returnvalue_3 0.0 1.0))
  (bind _returnvalue_6 (* _returnvalue_5 _returnvalue_4))
  (Utilities|FlowControl|Sequence
    (:then_0
      (if (or (!= (Input|AxisValues|GetMoveRight) 0.0) (!= (Input|AxisValues|GetMoveForward) 0.0))
        (Variables|Default|SetLast%20Right%20Value (Input|AxisValues|GetMoveRight))
        (Variables|Default|SetLast%20Up%20Value (Input|AxisValues|GetMoveForward))
        (if (not (Variables|Default|GetIs%20Shooting))
          (if (> (Math|Vector|VectorLength _returnvalue_6) 0.0)
            (Transformation|SetWorldRotation (Variables|Collision|GetCapsuleComponent) "0, 0, 0" false false)
            (Transformation|AddActorWorldOffset _returnvalue_6 true)
            (else
              (Pawn|Input|AddMovementInput "0, 0, 0" 1.0 false))))))
    (:then_1
      (bind _currentanimation (CallFunction|UpdateAnimation (Input|AxisValues|GetMoveRight) (* (Input|AxisValues|GetMoveForward) 1.0) (Variables|Default|GetLast%20Right%20Value) (* (Variables|Default|GetLast%20Up%20Value) 1.0)))
      (Sprite|SetFlipbook (Variables|Default|GetSprite) _currentanimation))
    (:then_2
      (if (Variables|Default|GetIs%20Shooting)
        (CallFunction|ShootProjectile (Math|Vector|MakeVector (Variables|Default|GetLast%20Right%20Value) 0.0 (Variables|Default|GetLast%20Up%20Value)))))))

(event Input|ActionEvents|InputActionShoot
  (params (Key :type Key%20Structure :default "AnyKey"))
  (:Pressed
    (Variables|Default|SetIs%20Shooting true)
    (CallFunction|ShootProjectile (Math|Vector|MakeVector (Variables|Default|GetLast%20Right%20Value) 0.0 (Variables|Default|GetLast%20Up%20Value))))
  (:Released
    (Variables|Default|SetIs%20Shooting false)))

(fn ConstructionScript)

(fn UpdateAnimation
  (params (Right%20Axis :type Float%20%28single-precision%29) (Up%20Axis :type Float%20%28single-precision%29) (Last%20Right :type Float%20%28single-precision%29) (Last%20Up :type Float%20%28single-precision%29))
  (LocalVariables|SetRightLocal Right%20Axis)
  (LocalVariables|SetUpLocal Up%20Axis)
  (LocalVariables|SetLastRightLocal Last%20Right)
  (LocalVariables|SetLastUpLocal Last%20Up)
  (Math|Float|CompareFloat (LocalVariables|GetRightLocal) 0.0
    (:>
      (Math|Float|CompareFloat (LocalVariables|GetUpLocal) 0.0
        (:>
          (LocalVariables|SetAnimationLocal "/Game/FlipBooks/Characters/Elf/Elf_NE.Elf_NE"))
        (:==
          (LocalVariables|SetAnimationLocal "/Game/FlipBooks/Characters/Elf/Elf_E.Elf_E"))
        (:<
          (LocalVariables|SetAnimationLocal "/Game/FlipBooks/Characters/Elf/Elf_SE.Elf_SE"))))
    (:==
      (Math|Float|CompareFloat (LocalVariables|GetUpLocal) 0.0
        (:>
          (LocalVariables|SetAnimationLocal "/Game/FlipBooks/Characters/Elf/Elf_N.Elf_N"))
        (:==
          (Math|Float|CompareFloat (LocalVariables|GetLastRightLocal) 0.0
            (:>
              (Math|Float|CompareFloat (LocalVariables|GetLastUpLocal) 0.0
                (:>
                  (LocalVariables|SetAnimationLocal "/Game/FlipBooks/Characters/Elf/Elf_NE_IDOL.Elf_NE_IDOL"))
                (:==
                  (LocalVariables|SetAnimationLocal "/Game/FlipBooks/Characters/Elf/Elf_E_IDOL.Elf_E_IDOL"))
                (:<
                  (LocalVariables|SetAnimationLocal "/Game/FlipBooks/Characters/Elf/Elf_SE_IDOL.Elf_SE_IDOL"))))
            (:==
              (Math|Float|CompareFloat (LocalVariables|GetLastUpLocal) 0.0
                (:>
                  (LocalVariables|SetAnimationLocal "/Game/FlipBooks/Characters/Elf/Elf_IDOL.Elf_IDOL"))
                (:==
                  ;[1 1 1] This is Start Animation
                  (LocalVariables|SetAnimationLocal "/Game/FlipBooks/Characters/Elf/Elf_S_IDOL.Elf_S_IDOL"))
                (:<
                  (LocalVariables|SetAnimationLocal "/Game/FlipBooks/Characters/Elf/Elf_S_IDOL.Elf_S_IDOL"))))
            (:<
              (Math|Float|CompareFloat (LocalVariables|GetLastUpLocal) 0.0
                (:>
                  (LocalVariables|SetAnimationLocal "/Game/FlipBooks/Characters/Elf/Elf_NW_IDOL.Elf_NW_IDOL"))
                (:==
                  (LocalVariables|SetAnimationLocal "/Game/FlipBooks/Characters/Elf/Elf_W_IDOL.Elf_W_IDOL"))
                (:<
                  (LocalVariables|SetAnimationLocal "/Game/FlipBooks/Characters/Elf/Elf_SW_IDOL.Elf_SW_IDOL"))))))
        (:<
          (LocalVariables|SetAnimationLocal "/Game/FlipBooks/Characters/Elf/Elf_S.Elf_S"))))
    (:<
      (Math|Float|CompareFloat (LocalVariables|GetUpLocal) 0.0
        (:>
          (LocalVariables|SetAnimationLocal "/Game/FlipBooks/Characters/Elf/Elf_NW.Elf_NW"))
        (:==
          (LocalVariables|SetAnimationLocal "/Game/FlipBooks/Characters/Elf/Elf_W.Elf_W"))
        (:<
          (LocalVariables|SetAnimationLocal "/Game/FlipBooks/Characters/Elf/Elf_SW.Elf_SW")))))
  (return (LocalVariables|GetAnimationLocal)))

(fn ShootProjectile
  (params (Direction :type Vector))
  (bind _returnvalue (Transformation|GetActorLocation))
  (bind _returnvalue_2 (Math|Conversions|RotationFromXVector Direction))
  (bind _gun_offset (Variables|Default|GetGun%20Offset))
  (bind _returnvalue_3 (Math|Vector|RotateVector _gun_offset _returnvalue_2))
  (bind _returnvalue_4 (+ _returnvalue _returnvalue_3))
  (if (Variables|Default|GetCan%20Fire)
    (if (> (Math|Vector|VectorLength Direction) 0.0)
      (Game|SpawnActorfromClass "/Game/Blueprints/Projectile.Projectile_C" (Math|Transform|MakeTransform _returnvalue_4 _returnvalue_2 "0.800000,0.800000,0.800000") "AlwaysSpawn" 0 0)
      (Audio|PlaySoundatLocation "/Game/Audio/fireelf.fireelf" _returnvalue_4)
      (Variables|Default|SetCan%20Fire false)
      (Utilities|Time|SetTimerbyFunctionName 0 "Shot Timer EXpired" (Variables|Default|GetFireRate)))))

(fn ShotTimerEXpired
  (Variables|Default|SetCan%20Fire true))