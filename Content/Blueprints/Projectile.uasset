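; Paper2D projectile actor that damages whatever it hits.
; On BeginPlay it copies its Damage value from the first Database actor found in the level.
; On hit it switches to the impact flipbook and, if that switch succeeds, waits briefly, destroys itself, then applies damage to the other actor.
; The damage call comes after DestroyActor in the chain.
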(event EventBeginPlay
  (bind _outactors (Actor|GetAllActorsOfClass "/Game/Blueprints/Database.Database_C"))
  (bind _output_get (Variables|Default|SetDamage (Variables|/Game/Blueprints/Database.Database_C|GetDamage (Utilities|Array|Get(acopy) _outactors)))))

(event Collision|EventHit
  (params (MyComp :type Primitive%20Component%20Object%20Reference) (Other :type Actor%20Object%20Reference) (OtherComp :type Primitive%20Component%20Object%20Reference) (bSelfMoved :type Boolean) (HitLocation :type Vector) (HitNormal :type Vector :default "0, 0, 0") (NormalImpulse :type Vector :default "0, 0, 0") (Hit :type Hit%20Result%20Structure%20%28by%20ref%29))
  (bind _projectileexplode (CallFunction|OnCollision))
  (if _projectileexplode
    (Utilities|FlowControl|Delay 0.1)
    (Actor|DestroyActor)
    (Game|Damage|ApplyDamage Other (stale EventBeginPlay _output_get) 0 self)))

(fn ConstructionScript)

(fn OnCollision
  (bind _returnvalue (Sprite|SetFlipbook (Variables|Default|GetPaperFlipbook) "/Game/FlipBooks/Effects/Projectile_Hit.Projectile_Hit"))
  (return _returnvalue))