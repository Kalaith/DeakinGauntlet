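; Destructible monster spawner with a flipbook sprite that periodically spawns monsters beside itself, up to a limit on living ones.
; A looping timer spawns the configured class, skipping blocked spots, and counts Ghosts or Demons.
; Their destroyed events are bound to lower the count; the death handler also plays a random sound.
; Projectile hits subtract GameInstance damage from spawner health; at zero, Tick shows an explosion flipbook and destroys it.
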(event EventBeginPlay
  ;[1 1 1] After play begins start spawning monsters
  (Utilities|Time|SetTimerbyFunctionName 0 "SpawnMonster" (Variables|Default|GetspawnRate) true))

(event EventTick
  (params (DeltaSeconds :type Float%20%28single-precision%29))
  ;[1 1 1] When the health of the spawn point is 0 or less destroy
  (Math|Integer|CompareInt (Variables|Default|GetspawnHealth) 0
    (:==
      _)
    (:<
      _))
  (Sprite|SetFlipbook (Variables|Default|GetPaperFlipbook) "/Game/FlipBooks/Effects/Explosion.Explosion")
  (Utilities|FlowControl|Delay 0.2)
  (Actor|DestroyActor))

(event Collision|EventHit
  (params (MyComp :type Primitive%20Component%20Object%20Reference) (Other :type Actor%20Object%20Reference) (OtherComp :type Primitive%20Component%20Object%20Reference) (bSelfMoved :type Boolean) (HitLocation :type Vector) (HitNormal :type Vector :default "0, 0, 0") (NormalImpulse :type Vector :default "0, 0, 0") (Hit :type Hit%20Result%20Structure%20%28by%20ref%29))
  (bind _asgame_instance_bp (Utilities|Casting|CastToGameInstance_BP (Game|GetGameInstance)))
  (Utilities|Casting|CastToProjectile Other)
  (Variables|Default|SetspawnHealth (- (Variables|Default|GetspawnHealth) (Math|Float|Floor (Variables|/Game/Blueprints/GameInstance_BP.GameInstance_BP_C|GetDamage _asgame_instance_bp)))))

(fn ConstructionScript
  (Sprite|SetFlipbook (Variables|Default|GetPaperFlipbook) (Variables|Default|GetspriteSpawner)))

(fn SpawnMonster
  (bind _self self)
  (bind _returnvalue (Transformation|GetActorTransform _self))
  (bind (_location _rotation _scale) (Math|Transform|BreakTransform _returnvalue))
  (bind (_x _y _z) (Math|Vector|BreakVector _location))
  ;[1 1 1] Limit the amount of monsters a spawner can spawn
  (Math|Integer|CompareInt (Variables|Default|GetmonstersSpawned) (Variables|Default|GetspawnLimit)
    (:>
      (Variables|Default|SetcanSpawn false :!label _label))
    (:==
      (goto _label))
    (:<
      (Variables|Default|SetcanSpawn true)))
  (if (Variables|Default|GetcanSpawn)
    (bind _returnvalue_2 (Game|SpawnActorfromClass (Variables|Default|GetspawnType) (Math|Transform|MakeTransform (Math|Vector|MakeVector (+ _x 25.0) _y _z) _rotation _scale) "AdjustIfPossibleButDontSpawnIfColliding" 0 0))
    ;[1 1 1] If the monster can spawn, assign an event on death to increse the spawner
    (if (Utilities|IsValid _returnvalue_2)
      (bind _asghosts_bp (Utilities|Casting|CastToGhosts_BP _returnvalue_2)
        (:then
          (EventDispatchers|BindEventtoMonsterDestroyed _asghosts_bp (EventDispatchers|CreateEvent :!event DestroyedMonster)))
        (:CastFailed
          (bind _asdemons_bp (Utilities|Casting|CastToDemons_BP _returnvalue_2))
          (EventDispatchers|BindEventtoMonsterDestroyed _asdemons_bp (EventDispatchers|CreateEvent :!event DestroyedMonster))))
      ;[1 1 1] Increase Spawn Counter by 1
      (Variables|Default|SetmonstersSpawned (+ (Variables|Default|GetmonstersSpawned) 1))
      ;[1 1 1] Limit the amount of monsters a spawner can spawn
      (Math|Integer|CompareInt (Variables|Default|GetmonstersSpawned) (Variables|Default|GetspawnLimit)
        (:>
          (Variables|Default|SetcanSpawn false :!label _label_2))
        (:==
          (goto _label_2))
        (:<
          (Variables|Default|SetcanSpawn true))))))

(fn DestroyedMonster
  (switch int (Math|Random|RandomInteger 3)
    (:Default
      (Audio|PlaySound2D "/Game/Audio/monsterdeath3.monsterdeath3"))
    (:0
      (Audio|PlaySound2D "/Game/Audio/monsterdeath1.monsterdeath1"))
    (:1
      (Audio|PlaySound2D "/Game/Audio/monsterdeath2.monsterdeath2")))
  ;[1 1 1] Reduce Spawn Counter by 1
  (Variables|Default|SetmonstersSpawned (- (Variables|Default|GetmonstersSpawned) 1))
  ;[1 1 1] Limit the amount of monsters a spawner can spawn
  (Math|Integer|CompareInt (Variables|Default|GetmonstersSpawned) (Variables|Default|GetspawnLimit)
    (:>
      (Variables|Default|SetcanSpawn false :!label _label))
    (:==
      (goto _label))
    (:<
      (Variables|Default|SetcanSpawn true))))